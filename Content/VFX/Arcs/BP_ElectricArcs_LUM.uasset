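; BP_ElectricArcs_LUM is an electric arc hazard or charger that raises the kart's electricity while it is inside the Zapping volume.
; Overlap events toggle InArea and start or fade out a charge sound.
; While the kart is inside, alive and below full charge, Tick shows the Niagara arc with its beam end tracking the kart mesh.
; A Delay on Tick throttles the charge increments; otherwise the arc is hidden.
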(event `self.ReceiveBeginPlay`
  (bind _returnvalue (`GameplayStatics.GetActorOfClass` "/Game/Blueprints/Kart/BP_Kart.BP_Kart_C"))
  (set `self.KartRef` _returnvalue))

(event `self.ReceiveTick`
  (params (DeltaSeconds :type "Float (single-precision)"))
  (bind _kartref (`self.KartRef`))
  (bind _electricarcs (`self.ElectricArcs`))
  (if (and (`self.InArea`) (< (`/Game/Blueprints/Kart/BP_Kart.ElectricityAmount` _kartref) 100.0) (`/Game/Blueprints/Kart/BP_Kart.isAlive` _kartref))
    (`|ExecutionSequence`
      (:`then_0`
        (`SceneComponent.SetHiddenInGame` _electricarcs false false)
        (`FXSystemComponent.SetVectorParameter` (`self.ElectricArcs`) "User.Beam End" (`SceneComponent.K2_GetComponentLocation` (`/Game/Blueprints/Kart/BP_Kart.KartMesh` (`self.KartRef`)))))
      (:`then_1`
        (`KismetSystemLibrary.Delay` (`self.TickTime`))
        (`/Game/Blueprints/Kart/BP_Kart.Increase Electricity` (`self.KartRef`) (`self.ChargePerTick`))))
    (else
      (`SceneComponent.SetHiddenInGame` _electricarcs true false))))

(event `self.Zapping.OnComponentBeginOverlap`
  (params (OverlappedComponent :type "PrimitiveComponent Object Reference") (OtherActor :type "Actor Object Reference") (OtherComp :type "PrimitiveComponent Object Reference") (OtherBodyIndex :type Integer) (bFromSweep :type Boolean) (SweepResult :type "HitResult Structure (by ref)"))
  (cast `/Game/Blueprints/Kart/BP_Kart` OtherActor)
  (set `self.InArea` true)
  (`AudioComponent.Play` (`self.ChargeCue`) 4.0))

(event `self.Zapping.OnComponentEndOverlap`
  (params (OverlappedComponent :type "PrimitiveComponent Object Reference") (OtherActor :type "Actor Object Reference") (OtherComp :type "PrimitiveComponent Object Reference") (OtherBodyIndex :type Integer))
  (cast `/Game/Blueprints/Kart/BP_Kart` OtherActor)
  (set `self.InArea` false)
  (`AudioComponent.FadeOut` (`self.ChargeCue`) 0.2 0.0 "Linear"))

(fn `UserConstructionScript`
  (`FXSystemComponent.SetVectorParameter` (`self.ElectricArcs`) "User.Beam End" (`SceneComponent.K2_GetComponentLocation` (`self.Start`))))