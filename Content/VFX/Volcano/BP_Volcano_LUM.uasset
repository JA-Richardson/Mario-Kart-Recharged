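; Volcano VFX actor that plays a timed eruption sequence once play begins.
; After successive delays, BeginPlay calls the Steam, Rumble and Explode events, escalating from steam to a large flaming, glowing blast.
; Each stage calls SetParameters, which pushes cloud, scale, lifetime, flame and glow float parameters to a single Smoke particle component.
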(event `self.ReceiveBeginPlay`
  (`KismetSystemLibrary.Delay` 5.0)
  (`self.Steam`)
  (`KismetSystemLibrary.Delay` 5.0)
  (`self.Rumble`)
  (`KismetSystemLibrary.Delay` 5.0)
  (`self.Explode`))

(event `Steam`
  (`self.Set Parameters` 15.0 2.0 3.0 6.0))

(event `Rumble`
  (`self.Set Parameters` 20.0 3.0 6.0 7.0 0.02))

(event `Explode`
  (`self.Set Parameters` 30.0 10.0 15.0 10.0 1.0 0.7))

(fn `Set Parameters`
  (params (Clouds :type "Float (double-precision)" :default 15.0) (`Min Scale` :type "Float (double-precision)" :default 1.0) (`Max Scale` :type "Float (double-precision)" :default 2.0) (Lifetime :type "Float (double-precision)" :default 5.0) (`Max Flame` :type "Float (double-precision)" :default 0.01) (Glow :type "Float (double-precision)" :default 1.0))
  (bind _smoke (`self.Smoke`))
  (`FXSystemComponent.SetFloatParameter` _smoke "Clouds" Clouds)
  (`FXSystemComponent.SetFloatParameter` _smoke "Min Scale" `Min Scale`)
  (`FXSystemComponent.SetFloatParameter` _smoke "Max Scale" `Max Scale`)
  (`FXSystemComponent.SetFloatParameter` _smoke "Lifetime" Lifetime)
  (`FXSystemComponent.SetFloatParameter` _smoke "Max Flame" `Max Flame`)
  (`FXSystemComponent.SetFloatParameter` _smoke "Glow" Glow))

(fn `UserConstructionScript`)