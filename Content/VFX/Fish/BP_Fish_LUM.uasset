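; Fish VFX actor that moves a skeletal mesh along its spline at a randomized speed.
; On BeginPlay it picks the FloatingPawnMovement max speed and divides spline length by it to set the timeline's play rate.
; Timeline alpha maps to distance along the spline, driving MoveComponentTo with local location and rotation.
; PlayFromStart follows that move within the Update branch, not Finished, restarting the timeline from there.
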(event `self.ReceiveBeginPlay`
  (bind _spline (`self.Spline`))
  (bind _returnvalue (`KismetMathLibrary.Lerp` 0.0 (`SplineComponent.GetSplineLength` _spline) (`self.Alpha`)))
  (bind _output_get (set `FloatingPawnMovement.MaxSpeed` (`KismetMathLibrary.RandomFloatInRange` 100.0 700.0) (`self.FloatingPawnMovement`)))
  (bind _output_get_2 (set `self.Duration` (/ (`SplineComponent.GetSplineLength` (`self.Spline`)) _output_get)))
  (`TimelineComponent.SetPlayRate` (`self.MoveTimeline`) (/ 1.0 _output_get_2))
  (bind (_direction _alpha) (`Timeline|MoveTimeline` :!label _label)
    (:`Update`
      (set `self.Alpha` _alpha)
      (`KismetSystemLibrary.MoveComponentTo` (`self.SkeletalMesh`) (`SplineComponent.GetLocationAtDistanceAlongSpline` _spline _returnvalue "Local") (`SplineComponent.GetRotationAtDistanceAlongSpline` _spline _returnvalue "Local"))
      (goto _label :!via `PlayFromStart`))))

(fn `UserConstructionScript`)