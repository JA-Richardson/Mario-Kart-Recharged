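; Spline-driven track generator that builds a chain of spline mesh segments in the construction script, optionally closed into a loop.
; GenerateColliders enables collision and switches segmentation from one piece per spline point to samples every Divisor units of length.
; TrackDataArray is resized to the segment count, supplying bank, width and thickness as each segment's start and end roll and scale.
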(fn `BuildTrackElement`
  (params (LoopIndex :type Integer) (TrackElementMesh :type "StaticMesh Object Reference"))
  (locals (Index :type Integer) (NextIndex :type Integer) (TrackElement :type "StaticMesh Object Reference") (StartLocation :type "Vector Structure") (StartTangent :type "Vector Structure") (EndLocation :type "Vector Structure") (EndTangent :type "Vector Structure") (CurrentSplineMesh :type "SplineMeshComponent Object Reference") (StartRoll :type "Float (double-precision)") (StartScale :type "Vector2D Structure") (EndRoll :type "Float (double-precision)") (EndScale :type "Vector2D Structure"))
  (bind _spline (`self.Spline`))
  (bind _spline_2 (`self.Spline`))
  (bind _returnvalue (* (`local.NextIndex`) (`self.Divisor`)))
  (bind _returnvalue_2 (* (`local.Index`) (`self.Divisor`)))
  (bind (_location _tangent) (`SplineComponent.GetLocationAndTangentAtSplinePoint` (`self.Spline`) (`local.NextIndex`) "Local"))
  (bind (_location_2 _tangent_2) (`SplineComponent.GetLocationAndTangentAtSplinePoint` (`self.Spline`) (`local.Index`) "Local"))
  (bind (_output_trackbank _output_trackwidth _output_trackthickness) (break `/Game/Blueprints/TrackSpline/S_TrackInfo` (`|GetArrayItem` (`self.TrackDataArray`) (`local.NextIndex`))))
  (bind (_output_trackbank_2 _output_trackwidth_2 _output_trackthickness_2) (break `/Game/Blueprints/TrackSpline/S_TrackInfo` (`|GetArrayItem` (`self.TrackDataArray`) (`local.Index`))))
  (set `local.Index` LoopIndex)
  (if (`self.Loop`)
    (set `local.NextIndex` (mod (+ LoopIndex 1) (`self.NumberOfSplinePoints`)))
    (else
      (set `local.NextIndex` (`KismetMathLibrary.Clamp` (+ LoopIndex 1) 0 (`self.NumberOfSplinePoints`)))))
  (set `local.TrackElement` TrackElementMesh)
  (`|ExecutionSequence`
    (:`then_0`
      (if (`self.GenerateColliders`)
        (set `local.StartLocation` (`SplineComponent.GetLocationAtDistanceAlongSpline` _spline_2 _returnvalue_2 "Local"))
        (set `local.StartTangent` (`SplineComponent.GetTangentAtDistanceAlongSpline` _spline_2 _returnvalue_2 "Local"))
        (set `local.EndLocation` (`SplineComponent.GetLocationAtDistanceAlongSpline` _spline _returnvalue "Local"))
        (set `local.EndTangent` (`SplineComponent.GetTangentAtDistanceAlongSpline` _spline _returnvalue "Local"))
        (else
          (set `local.StartLocation` _location_2)
          (set `local.StartTangent` _tangent_2)
          (set `local.EndLocation` _location)
          (set `local.EndTangent` _tangent)))
      (set `local.StartRoll` _output_trackbank_2)
      (set `local.StartScale` (`KismetMathLibrary.MakeVector2D` _output_trackwidth_2 _output_trackthickness_2))
      (set `local.EndRoll` _output_trackbank)
      (set `local.EndScale` (`KismetMathLibrary.MakeVector2D` _output_trackwidth _output_trackthickness)))
    (:`then_1`
      (bind _returnvalue_3 (`AddComponent|NODE_AddSplineMeshComponent-0`))
      (set `local.CurrentSplineMesh` _returnvalue_3)
      (`StaticMeshComponent.SetStaticMesh` (`local.CurrentSplineMesh`) (`local.TrackElement`))
      (`SplineMeshComponent.SetStartAndEnd` (`local.CurrentSplineMesh`) (`local.StartLocation`) (`local.StartTangent`) (`local.EndLocation`) (`local.EndTangent`) true)
      (`SplineMeshComponent.SetStartRoll` (`local.CurrentSplineMesh`) (`local.StartRoll`) true)
      (`SplineMeshComponent.SetEndRoll` (`local.CurrentSplineMesh`) (`local.EndRoll`) true)
      (`SplineMeshComponent.SetStartScale` (`local.CurrentSplineMesh`) (`local.StartScale`) true)
      (`SplineMeshComponent.SetEndScale` (`local.CurrentSplineMesh`) (`local.EndScale`) true)
      (`PrimitiveComponent.SetCollisionEnabled` (`local.CurrentSplineMesh`) (`self.Collision`)))))

(fn `UserConstructionScript`
  (bind _trackdataarray (`self.TrackDataArray`))
  (if (`self.GenerateColliders`)
    (set `self.Collision` "QueryAndPhysics")
    (else
      (set `self.Collision` "NoCollision")))
  (`|ExecutionSequence`
    (:`then_0`
      (if (`self.GenerateColliders`)
        (set `self.NumberOfSplinePoints` (`.ReturnValue` (`KismetMathLibrary.FMod` (`SplineComponent.GetSplineLength` (`self.Spline`)) (`self.Divisor`))))
        (else
          (set `self.NumberOfSplinePoints` (`SplineComponent.GetNumberOfSplinePoints` (`self.Spline`))))))
    (:`then_1`
      (`/Engine/EditorBlueprintResources/StandardMacros.CompareInt` (`KismetArrayLibrary.Array_Length` (`self.TrackDataArray`)) (`self.NumberOfSplinePoints`) :!label _label
        (:`>`
          (`KismetArrayLibrary.Array_Remove` _trackdataarray (`KismetArrayLibrary.Array_LastIndex` _trackdataarray))
          (goto _label))
        (:`<`
          (`KismetArrayLibrary.Array_Add` (`self.TrackDataArray`))
          (goto _label))))
    (:`then_2`
      (for _index (range (`self.NumberOfSplinePoints`))
        (`self.BuildTrackElement` _index (`self.TrackMesh`))))))