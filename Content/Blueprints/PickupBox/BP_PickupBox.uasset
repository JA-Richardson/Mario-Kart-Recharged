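; BP_PickupBox is a spinning item box that grants a pickup to a BP_Kart overlapping its hitbox.
; While active, it plays a collect cue with a fade-out and calls the kart's CollectPickup through CollectRandomPickup.
; Any kart overlap then deactivates the box and hides its meshes until a Cooldown delay restores it.
; Tick rotates the Hitbox by a fixed per-frame step, so spin speed depends on frame rate.
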(event `self.ReceiveTick`
  (params (DeltaSeconds :type "Float (single-precision)"))
  ;[0.3005 0 1] Razvan Ivan - A0001151
  (`SceneComponent.K2_AddWorldRotation` (`self.Hitbox`) (struct :`Yaw` 1.0) false false))

(event `self.Hitbox.OnComponentBeginOverlap`
  (params (OverlappedComponent :type "PrimitiveComponent Object Reference") (OtherActor :type "Actor Object Reference") (OtherComp :type "PrimitiveComponent Object Reference") (OtherBodyIndex :type Integer) (bFromSweep :type Boolean) (SweepResult :type "HitResult Structure (by ref)"))
  (bind _itemcollect_cue (`self.itemCollect_Cue`))
  ;[0.3005 0 1] Razvan Ivan - A0001151
  (bind _asbp_kart (cast `/Game/Blueprints/Kart/BP_Kart` OtherActor))
  (`|ExecutionSequence`
    (:`then_0`
      (if (`self.isActive`)
        (`AudioComponent.Play` _itemcollect_cue 2.0)
        (`AudioComponent.FadeOut` _itemcollect_cue 1.0 0.0 "Linear")
        (`self.CollectRandomPickup` _asbp_kart)))
    (:`then_1`
      (bind _output_get (set `self.isActive` false))
      (`self.SetVisibility` _output_get)
      (`KismetSystemLibrary.Delay` (`self.Cooldown`))
      (bind _output_get_2 (set `self.isActive` true))
      (`self.SetVisibility` _output_get_2))))

(fn `CollectRandomPickup`
  (params (Kart :type "/Game/Blueprints/Kart/BP_Kart Object Reference"))
  (returns (Result :type Boolean))
  ;[0.3005 0 1] Razvan Ivan - A0001151
  (bind _success (`/Game/Blueprints/Kart/BP_Kart.CollectPickup` Kart))
  (return (not _success)))

(fn `SetVisibility`
  (params (Visibility :type Boolean))
  ;[0.3005 0 1] Razvan Ivan - A0001151
  (`SceneComponent.SetVisibility` (`self.Mesh`) Visibility true)
  (`SceneComponent.SetVisibility` (`self.Cylinder`) Visibility true))

(fn `UserConstructionScript`)