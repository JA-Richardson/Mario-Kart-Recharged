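; Start-line checkpoint actor for the kart track that advances a kart's lap count.
; When a BP_Kart overlaps the Checkpoint component and its checkpoint index matches CheckpointNum, both its checkpoint and lap counters increment.
; It also saves the component's world location and rotation on the kart as its last checkpoint transform.
; The construction script displays CheckpointNum on the Number text.
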(event `self.Checkpoint.OnComponentBeginOverlap`
  (params (OverlappedComponent :type "PrimitiveComponent Object Reference") (OtherActor :type "Actor Object Reference") (OtherComp :type "PrimitiveComponent Object Reference") (OtherBodyIndex :type Integer) (bFromSweep :type Boolean) (SweepResult :type "HitResult Structure (by ref)"))
  (bind _checkpoint (`self.Checkpoint`))
  (bind _asbp_kart (cast `/Game/Blueprints/Kart/BP_Kart` OtherActor))
  (bind _checkpoint_2 (`/Game/Blueprints/Kart/BP_Kart.Checkpoint` _asbp_kart))
  (if (== _checkpoint_2 (`self.CheckpointNum`))
    (set `/Game/Blueprints/Kart/BP_Kart.Checkpoint` (+ _checkpoint_2 1) _asbp_kart)
    (set `/Game/Blueprints/Kart/BP_Kart.Lap` (+ (`/Game/Blueprints/Kart/BP_Kart.Lap` _asbp_kart) 1) _asbp_kart)
    (set `/Game/Blueprints/Kart/BP_Kart.LastCPPos` (`SceneComponent.K2_GetComponentLocation` _checkpoint) _asbp_kart)
    (set `/Game/Blueprints/Kart/BP_Kart.LastCPRot` (`SceneComponent.K2_GetComponentRotation` _checkpoint) _asbp_kart)))

(fn `UserConstructionScript`
  (`TextRenderComponent.K2_SetText` (`self.Number`) (`KismetTextLibrary.Conv_IntToText` (`self.CheckpointNum`))))