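; Numbered track checkpoint that tracks BP_Kart race progress.
; An overlapping kart whose counter matches CheckpointNum advances it and stores the checkpoint's position and rotation.
; Node 0 otherwise adds a lap and resets the counter if it equals PreviousCheckpoint + 1.
; Construction shows the number and skips node 0 when deriving PreviousCheckpoint, but Tick overwrites it with CheckpointNum - 1 on every node, defeating that lap check.
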(event `self.Checkpoint.OnComponentBeginOverlap`
  (params (OverlappedComponent :type "PrimitiveComponent Object Reference") (OtherActor :type "Actor Object Reference") (OtherComp :type "PrimitiveComponent Object Reference") (OtherBodyIndex :type Integer) (bFromSweep :type Boolean) (SweepResult :type "HitResult Structure (by ref)"))
  (bind _checkpoint (`/Game/Blueprints/Kart/BP_Kart.Checkpoint` (`self.Kart`)))
  ;[1 1 1] Set CheckpointNum to corresponding position on the track
  (bind _asbp_kart (cast `/Game/Blueprints/Kart/BP_Kart` OtherActor))
  (set `self.Kart` _asbp_kart)
  (if (== _checkpoint (`self.CheckpointNum`))
    (set `/Game/Blueprints/Kart/BP_Kart.Checkpoint` (+ _checkpoint 1) (`self.Kart`))
    (set `/Game/Blueprints/Kart/BP_Kart.LastCPPos` (`SceneComponent.K2_GetComponentLocation` (`self.Checkpoint`)) (`self.Kart`))
    (set `/Game/Blueprints/Kart/BP_Kart.LastCPRot` (`SceneComponent.K2_GetComponentRotation` (`self.Checkpoint`)) (`self.Kart`))
    (elif (and (== (`self.CheckpointNum`) 0) (== (`/Game/Blueprints/Kart/BP_Kart.Checkpoint` (`self.Kart`)) (+ (`self.PreviousCheckpoint`) 1)))
      (set `/Game/Blueprints/Kart/BP_Kart.Checkpoint` 0 (`self.Kart`))
      (set `/Game/Blueprints/Kart/BP_Kart.Lap` (+ (`/Game/Blueprints/Kart/BP_Kart.Lap` (`self.Kart`)) 1) (`self.Kart`)))))

(event `self.ReceiveTick`
  (params (DeltaSeconds :type "Float (single-precision)"))
  (set `self.PreviousCheckpoint` (- (`self.CheckpointNum`) 1)))

(fn `UserConstructionScript`
  (`TextRenderComponent.K2_SetText` (`self.CheckpointNumber`) (`KismetTextLibrary.Conv_IntToText` (`self.CheckpointNum`)))
  (if (!= (`self.CheckpointNum`) 0)
    (set `self.PreviousCheckpoint` (- (`self.CheckpointNum`) 1))))