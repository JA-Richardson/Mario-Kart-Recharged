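; Thunder cloud actor that follows a target kart and strikes it with a timed stun.
; On BeginPlay and every Tick, it snaps its root to the kart's location and rotation.
; After a short delay, BeginPlay activates the Niagara effect and calls StunKart on the kart, then destroys the actor once a second delay ends.
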(event `self.ReceiveBeginPlay`
  ;[0.3005 0 1] Razvan Ivan - A0001151
  (`SceneComponent.K2_SetWorldLocationAndRotation` (`self.DefaultSceneRoot`) (.location (`/Game/Blueprints/Kart/BP_Kart.GetKartTransform` (`self.Kart`))) (.rotation (`/Game/Blueprints/Kart/BP_Kart.GetKartTransform` (`self.Kart`))) false false)
  (`KismetSystemLibrary.Delay` 3.0)
  (`ActorComponent.Activate` (`self.Niagara`) true)
  (`/Game/Blueprints/Kart/BP_Kart.StunKart` (`self.Kart`) 3.0)
  (`KismetSystemLibrary.Delay` 2.0)
  (`self.K2_DestroyActor`))

(event `self.ReceiveTick`
  (params (DeltaSeconds :type "Float (single-precision)"))
  ;[0.3005 0 1] Razvan Ivan - A0001151
  (`SceneComponent.K2_SetWorldLocationAndRotation` (`self.DefaultSceneRoot`) (.location (`/Game/Blueprints/Kart/BP_Kart.GetKartTransform` (`self.Kart`))) (.rotation (`/Game/Blueprints/Kart/BP_Kart.GetKartTransform` (`self.Kart`))) false false))

(fn `UserConstructionScript`)