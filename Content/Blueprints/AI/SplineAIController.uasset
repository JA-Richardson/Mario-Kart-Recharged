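; AI controller that drives a kart along the track in a racing game.
; Each tick, if the kart is valid, it applies a random throttle between moderate and full to move it.
; It gathers all TrackSplineNew actors, asks the kart for a track-following steering value, and steers with that value doubled.
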(event `self.ReceiveTick`
  (params (DeltaSeconds :type "Float (single-precision)"))
  (`/Engine/EditorBlueprintResources/StandardMacros.IsValid` (`self.Kart`)
    (:`Is Valid`
      (`/Game/Blueprints/Kart/BP_Kart.MoveKart` (`self.Kart`) (`KismetMathLibrary.RandomFloatInRange` 0.7 1.0))
      (bind _outactors (`GameplayStatics.GetAllActorsOfClass` "/Game/Blueprints/AI/TrackSplineNew.TrackSplineNew_C"))
      (bind _steering (`/Game/Blueprints/Kart/BP_Kart.AIGetTrack` (`self.Kart`) _outactors))
      (`/Game/Blueprints/Kart/BP_Kart.SteerKart` (`self.Kart`) (* _steering 2.0)))))

(fn `UserConstructionScript`)