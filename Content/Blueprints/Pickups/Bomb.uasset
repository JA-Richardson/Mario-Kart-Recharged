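; Bomb actor for a kart game that explodes three seconds after it spawns.
; A timer started on BeginPlay calls Detonate, which spawns a BombExplo actor at the bomb's transform and destroys the bomb.
; When Sphere1 overlaps any BP_Kart other than the stored Kart reference, the physics Sphere's linear velocity is zeroed, stopping the bomb without detonating it early.
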(event `self.ReceiveBeginPlay`
  (`KismetSystemLibrary.K2_SetTimerDelegate` (delegate `Detonate`) 3.0))

(event `Detonate`
  (`|SpawnActorFromClass` "/Game/Blueprints/Pickups/BombExplo.BombExplo_C" (`self.GetTransform`) "Undefined" "OverrideRootScale" null null)
  (`self.K2_DestroyActor`))

(event `self.Sphere1.OnComponentBeginOverlap`
  (params (OverlappedComponent :type "PrimitiveComponent Object Reference") (OtherActor :type "Actor Object Reference") (OtherComp :type "PrimitiveComponent Object Reference") (OtherBodyIndex :type Integer) (bFromSweep :type Boolean) (SweepResult :type "HitResult Structure (by ref)"))
  (bind _asbp_kart (cast `/Game/Blueprints/Kart/BP_Kart` OtherActor))
  (if (!= _asbp_kart (`self.Kart`))
    (`PrimitiveComponent.SetPhysicsLinearVelocity` (`self.Sphere`) (0.0 0.0 0.0) false "None")))

(fn `UserConstructionScript`)