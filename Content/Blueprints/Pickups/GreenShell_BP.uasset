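; GreenShell_BP is a kart-racing green shell item that destroys itself six seconds after spawning.
; Its sphere overlap checks the other actor in sequence against karts, bananas and false walls.
; It stuns any kart other than the one in its Kart variable, destroys bananas or despawns false walls, then destroys itself after each hit.
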(event `self.ReceiveBeginPlay`
  (`KismetSystemLibrary.Delay` 6.0)
  (`self.K2_DestroyActor`))

(event `self.SphereCollision.OnComponentBeginOverlap`
  (params (OverlappedComponent :type "PrimitiveComponent Object Reference") (OtherActor :type "Actor Object Reference") (OtherComp :type "PrimitiveComponent Object Reference") (OtherBodyIndex :type Integer) (bFromSweep :type Boolean) (SweepResult :type "HitResult Structure (by ref)"))
  (`|ExecutionSequence`
    (:`then_0`
      (bind _asbp_kart (cast `/Game/Blueprints/Kart/BP_Kart` OtherActor))
      (if (!= (`self.Kart`) _asbp_kart)
        (`/Game/Blueprints/Kart/BP_Kart.StunKart` _asbp_kart 2.0)
        (`self.K2_DestroyActor`)))
    (:`then_1`
      (bind _asbanana (cast `/Game/Blueprints/Pickups/Banana` OtherActor))
      (`self.K2_DestroyActor` _asbanana)
      (`self.K2_DestroyActor`))
    (:`then_2`
      (bind _asfalse_wall (cast `/Game/Blueprints/Pickups/FalseWall` OtherActor))
      (`/Game/Blueprints/Pickups/FalseWall.Despawn` _asfalse_wall)
      (`self.K2_DestroyActor`))))

(fn `UserConstructionScript`)