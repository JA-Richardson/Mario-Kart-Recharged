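; Triple-item pickup actor for the kart game that orbits shells, bananas or mushrooms around the player's kart.
; Tick pins it above player 0 while a Timeline spins three spring arms 120 degrees apart.
; UseTripleItem steps a counter: first use sets meshes and enables colliders, later uses hide items and update the kart's pickup, the last destroys the actor.
; Collider overlaps stun karts or remove targets, bananas and false walls, consuming an item.
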(event `self.Collision1.OnComponentBeginOverlap`
  (params (OverlappedComponent :type "PrimitiveComponent Object Reference") (OtherActor :type "Actor Object Reference") (OtherComp :type "PrimitiveComponent Object Reference") (OtherBodyIndex :type Integer) (bFromSweep :type Boolean) (SweepResult :type "HitResult Structure (by ref)"))
  ;[1 1 1] Collision While Spinning
  (bind _asbp_kart (cast `/Game/Blueprints/Kart/BP_Kart` OtherActor)
    (:`then`
      (`/Game/Blueprints/Kart/BP_Kart.StunKart` _asbp_kart 2.0))
    (:`CastFailed`
      (bind _astarget_kart (cast `/Game/Blueprints/Pickups/TargetKart` OtherActor)
        (:`then`
          (`self.K2_DestroyActor` _astarget_kart))
        (:`CastFailed`
          (bind _asbanana (cast `/Game/Blueprints/Pickups/Banana` OtherActor)
            (:`then`
              (`self.K2_DestroyActor` _asbanana))
            (:`CastFailed`
              (bind _asfalse_wall (cast `/Game/Blueprints/Pickups/FalseWall` OtherActor))
              (`/Game/Blueprints/Pickups/FalseWall.Despawn` _asfalse_wall)))))))
  (`self.UseTripleItem` "NewEnumerator0"))

(event `self.ReceiveTick`
  (params (DeltaSeconds :type "Float (single-precision)"))
  ;[1 1 1] Stay on User
  (`self.K2_SetActorLocation` (+ (`self.K2_GetActorLocation` (`GameplayStatics.GetPlayerCharacter` 0)) (0.0 0.0 75.0)) false true))

(event `self.ReceiveBeginPlay`
  ;[1 1 1] TripleShellSetUp
  (`SceneComponent.SetVisibility` (`self.Object1`) false false)
  (`SceneComponent.SetVisibility` (`self.Object2`) false false)
  (`SceneComponent.SetVisibility` (`self.Object3`) false false)
  (`PrimitiveComponent.SetCollisionEnabled` (`self.Collision2`) "NoCollision")
  (`PrimitiveComponent.SetCollisionEnabled` (`self.Collision3`) "NoCollision")
  (`PrimitiveComponent.SetCollisionEnabled` (`self.Collision1`) "NoCollision")
  (bind (_direction _newtrack_0) (`Timeline|Timeline_0`)
    (:`Update`
      (`SceneComponent.K2_SetRelativeRotation` (`self.SpringArm`) (`self.Object Rotator` _newtrack_0 120.0) false false)
      (`SceneComponent.K2_SetRelativeRotation` (`self.SpringArm1`) (`self.Object Rotator` _newtrack_0 240.0) false false)
      (`SceneComponent.K2_SetRelativeRotation` (`self.SpringArm2`) (`self.Object Rotator` _newtrack_0 360.0) false false))))

(event `self.Collision2.OnComponentBeginOverlap`
  (params (OverlappedComponent :type "PrimitiveComponent Object Reference") (OtherActor :type "Actor Object Reference") (OtherComp :type "PrimitiveComponent Object Reference") (OtherBodyIndex :type Integer) (bFromSweep :type Boolean) (SweepResult :type "HitResult Structure (by ref)"))
  ;[1 1 1] Collision While Spinning
  (bind _asbp_kart (cast `/Game/Blueprints/Kart/BP_Kart` OtherActor)
    (:`then`
      (`/Game/Blueprints/Kart/BP_Kart.StunKart` _asbp_kart 2.0))
    (:`CastFailed`
      (bind _astarget_kart (cast `/Game/Blueprints/Pickups/TargetKart` OtherActor)
        (:`then`
          (`self.K2_DestroyActor` _astarget_kart))
        (:`CastFailed`
          (bind _asbanana (cast `/Game/Blueprints/Pickups/Banana` OtherActor)
            (:`then`
              (`self.K2_DestroyActor` _asbanana))
            (:`CastFailed`
              (bind _asfalse_wall (cast `/Game/Blueprints/Pickups/FalseWall` OtherActor))
              (`/Game/Blueprints/Pickups/FalseWall.Despawn` _asfalse_wall)))))))
  (`self.UseTripleItem` "NewEnumerator0"))

(event `UseTripleItem`
  (params (Type :type "/Game/Blueprints/Pickups/TripleEnum Enum" :default "NewEnumerator0"))
  (bind _array (`|MakeArray` (`self.Object1`) (`self.Object2`) (`self.Object3`)))
  ;[1 1 1] UseingTripleItems
  (switch `int` (`self.TripleItemTracker`)
    (:`0`
      ;;[1 1 1] First Use
      (bind _output_get (set `self.Type` Type))
      (switch `/Game/Blueprints/Pickups/TripleEnum` _output_get
        (:`NewEnumerator0`
          (for _array_element _array
            (`StaticMeshComponent.SetStaticMesh` _array_element "/Game/SM_RedKoopaShell.SM_RedKoopaShell")
            (`SceneComponent.SetWorldScale3D` (stale _array_element_2) (15.0 15.0 15.0) :!label _label)
            (`SceneComponent.SetWorldScale3D` _array_element (15.0 15.0 15.0))))
        (:`NewEnumerator1`
          (for _array_element_2 _array
            (`StaticMeshComponent.SetStaticMesh` _array_element_2 "/Game/BlockoutTests/SM_GreenKoopaShell.SM_GreenKoopaShell")
            (goto _label)))
        (:`NewEnumerator2`
          (for _array_element_3 _array
            (`StaticMeshComponent.SetStaticMesh` _array_element_3 "/Game/BlockoutTests/SM_Banana.SM_Banana")
            (`SceneComponent.SetWorldScale3D` _array_element_3 (10.0 10.0 10.0))))
        (:`NewEnumerator3`
          (for _array_element_4 _array
            (`StaticMeshComponent.SetStaticMesh` _array_element_4 "/Game/BlockoutTests/SM_Mushroom.SM_Mushroom")
            (`SceneComponent.SetWorldScale3D` _array_element_4 (15.0 15.0 15.0)))))
      (`SceneComponent.SetVisibility` (`self.Object1`) true true)
      (`SceneComponent.SetVisibility` (`self.Object2`) true true)
      (`SceneComponent.SetVisibility` (`self.Object3`) true true)
      (`PrimitiveComponent.SetCollisionEnabled` (`self.Collision2`) "QueryOnly")
      (`PrimitiveComponent.SetCollisionEnabled` (`self.Collision3`) "QueryOnly")
      (`PrimitiveComponent.SetCollisionEnabled` (`self.Collision1`) "QueryOnly")
      (`/Engine/EditorBlueprintResources/StandardMacros.IncrementInt` (`self.TripleItemTracker`)
        (:`  `
          (bind _asbp_kart (cast `/Game/Blueprints/Kart/BP_Kart` (`GameplayStatics.GetPlayerCharacter` 0)))
          (switch `/Game/Blueprints/Pickups/TripleEnum` (`self.Type`)
            (:`NewEnumerator0`
              (set `/Game/Blueprints/Kart/BP_Kart.PickupMain` "NewEnumerator18" _asbp_kart))
            (:`NewEnumerator1`
              (set `/Game/Blueprints/Kart/BP_Kart.PickupMain` "NewEnumerator12" _asbp_kart))
            (:`NewEnumerator2`
              (set `/Game/Blueprints/Kart/BP_Kart.PickupMain` "NewEnumerator14" _asbp_kart))
            (:`NewEnumerator3`
              (set `/Game/Blueprints/Kart/BP_Kart.PickupMain` "NewEnumerator20" _asbp_kart)))
          (set `/Game/Blueprints/Kart/BP_Kart.TripleActive` true _asbp_kart))))
    (:`1`
      ;;[1 1 1] 3 Items
      (`SceneComponent.SetVisibility` (`self.Object1`) false true)
      (`PrimitiveComponent.SetCollisionEnabled` (`self.Collision1`) "NoCollision")
      (`/Engine/EditorBlueprintResources/StandardMacros.IncrementInt` (`self.TripleItemTracker`)
        (:`  `
          (bind _asbp_kart_2 (cast `/Game/Blueprints/Kart/BP_Kart` (`GameplayStatics.GetPlayerCharacter` 0)))
          (switch `/Game/Blueprints/Pickups/TripleEnum` (`self.Type`)
            (:`NewEnumerator0`
              (set `/Game/Blueprints/Kart/BP_Kart.PickupMain` "NewEnumerator17" _asbp_kart_2))
            (:`NewEnumerator1`
              (set `/Game/Blueprints/Kart/BP_Kart.PickupMain` "NewEnumerator11" _asbp_kart_2))
            (:`NewEnumerator2`
              (set `/Game/Blueprints/Kart/BP_Kart.PickupMain` "NewEnumerator13" _asbp_kart_2))
            (:`NewEnumerator3`
              (set `/Game/Blueprints/Kart/BP_Kart.PickupMain` "NewEnumerator19" _asbp_kart_2))))))
    (:`2`
      ;;[1 1 1] 2 Items
      (`SceneComponent.SetVisibility` (`self.Object2`) false true)
      (`PrimitiveComponent.SetCollisionEnabled` (`self.Collision2`) "NoCollision")
      (`/Engine/EditorBlueprintResources/StandardMacros.IncrementInt` (`self.TripleItemTracker`)
        (:`  `
          (bind _asbp_kart_3 (cast `/Game/Blueprints/Kart/BP_Kart` (`GameplayStatics.GetPlayerCharacter` 0)))
          (switch `/Game/Blueprints/Pickups/TripleEnum` (`self.Type`)
            (:`NewEnumerator0`
              (set `/Game/Blueprints/Kart/BP_Kart.PickupMain` "NewEnumerator0" _asbp_kart_3))
            (:`NewEnumerator1`
              (set `/Game/Blueprints/Kart/BP_Kart.PickupMain` "NewEnumerator1" _asbp_kart_3))
            (:`NewEnumerator2`
              (set `/Game/Blueprints/Kart/BP_Kart.PickupMain` "NewEnumerator8" _asbp_kart_3))
            (:`NewEnumerator3`
              (set `/Game/Blueprints/Kart/BP_Kart.PickupMain` "NewEnumerator3" _asbp_kart_3))))))
    (:`3`
      ;;[1 1 1] Last Item
      (`SceneComponent.SetVisibility` (`self.Object2`) false true)
      (`PrimitiveComponent.SetCollisionEnabled` (`self.Collision2`) "NoCollision")
      (`/Engine/EditorBlueprintResources/StandardMacros.IncrementInt` (`self.TripleItemTracker`)
        (:`  `
          (bind _asbp_kart_4 (cast `/Game/Blueprints/Kart/BP_Kart` (`GameplayStatics.GetPlayerCharacter` 0)))
          (switch `/Game/Blueprints/Pickups/TripleEnum` (`self.Type`)
            (:`NewEnumerator0`
              (set `/Game/Blueprints/Kart/BP_Kart.PickupMain` "NewEnumerator2" _asbp_kart_4))
            (:`NewEnumerator1`
              (set `/Game/Blueprints/Kart/BP_Kart.PickupMain` "NewEnumerator2" _asbp_kart_4))
            (:`NewEnumerator2`
              (set `/Game/Blueprints/Kart/BP_Kart.PickupMain` "NewEnumerator2" _asbp_kart_4))
            (:`NewEnumerator3`
              (set `/Game/Blueprints/Kart/BP_Kart.PickupMain` "NewEnumerator2" _asbp_kart_4)))
          (set `/Game/Blueprints/Kart/BP_Kart.TripleActive` false _asbp_kart_4)
          (`self.K2_DestroyActor`))))))

(event `self.Collision3.OnComponentBeginOverlap`
  (params (OverlappedComponent :type "PrimitiveComponent Object Reference") (OtherActor :type "Actor Object Reference") (OtherComp :type "PrimitiveComponent Object Reference") (OtherBodyIndex :type Integer) (bFromSweep :type Boolean) (SweepResult :type "HitResult Structure (by ref)"))
  ;[1 1 1] Collision While Spinning
  (bind _asbp_kart (cast `/Game/Blueprints/Kart/BP_Kart` OtherActor)
    (:`then`
      (`/Game/Blueprints/Kart/BP_Kart.StunKart` _asbp_kart 2.0))
    (:`CastFailed`
      (bind _astarget_kart (cast `/Game/Blueprints/Pickups/TargetKart` OtherActor)
        (:`then`
          (`self.K2_DestroyActor` _astarget_kart))
        (:`CastFailed`
          (bind _asbanana (cast `/Game/Blueprints/Pickups/Banana` OtherActor)
            (:`then`
              (`self.K2_DestroyActor` _asbanana))
            (:`CastFailed`
              (bind _asfalse_wall (cast `/Game/Blueprints/Pickups/FalseWall` OtherActor))
              (`/Game/Blueprints/Pickups/FalseWall.Despawn` _asfalse_wall)))))))
  (`self.UseTripleItem` "NewEnumerator0"))

(fn `UserConstructionScript`)