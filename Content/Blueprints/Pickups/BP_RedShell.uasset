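; Red shell projectile for a kart game that homes in on a target and destroys itself after six seconds.
; A detection radius collects hittable TargetKarts and locks projectile homing onto the first one, once.
; Its collision sphere stuns karts other than its own Kart, or removes bananas, false walls and TargetKarts, destroying the shell.
; A FindTarget function picks the nearest "Homing"-tagged actor but is not called in these graphs.
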(event `self.DetectionRadius.OnComponentBeginOverlap`
  (params (OverlappedComponent :type "PrimitiveComponent Object Reference") (OtherActor :type "Actor Object Reference") (OtherComp :type "PrimitiveComponent Object Reference") (OtherBodyIndex :type Integer) (bFromSweep :type Boolean) (SweepResult :type "HitResult Structure (by ref)"))
  (bind _targetstohit (`self.TargetsToHit`))
  ;[1 1 1] Collision event to detect target
  (bind _astarget_kart (cast `/Game/Blueprints/Pickups/TargetKart` OtherActor))
  (if (`/Game/Blueprints/Pickups/TargetKart.AbletoHit?` _astarget_kart)
    (`KismetArrayLibrary.Array_Add` _targetstohit _astarget_kart)
    (`/Engine/EditorBlueprintResources/StandardMacros.DoOnce` false
      (:`Completed`
        ;[1 1 1] Home to initial target
        (bind _astarget_kart_2 (cast `/Game/Blueprints/Pickups/TargetKart` (`|GetArrayItem` _targetstohit)))
        (set `ProjectileMovementComponent.HomingTargetComponent` (`/Game/Blueprints/Pickups/TargetKart.HomingTargetLocation` _astarget_kart_2) (`self.ProjectileMovement`))))))

(event `self.ReceiveBeginPlay`
  (`|ExecutionSequence`
    (:`then_0`
      (`KismetSystemLibrary.Delay` 6.0)
      (`self.K2_DestroyActor`))))

(event `self.SphereCollision.OnComponentBeginOverlap`
  (params (OverlappedComponent :type "PrimitiveComponent Object Reference") (OtherActor :type "Actor Object Reference") (OtherComp :type "PrimitiveComponent Object Reference") (OtherBodyIndex :type Integer) (bFromSweep :type Boolean) (SweepResult :type "HitResult Structure (by ref)"))
  (`|ExecutionSequence`
    (:`then_0`
      (bind _asbp_kart (cast `/Game/Blueprints/Kart/BP_Kart` OtherActor))
      (if (!= (`self.Kart`) _asbp_kart)
        (`/Game/Blueprints/Kart/BP_Kart.StunKart` _asbp_kart 2.0)
        (`self.K2_DestroyActor`)))
    (:`then_1`
      (bind _asbanana (cast `/Game/Blueprints/Pickups/Banana` OtherActor))
      (`self.K2_DestroyActor` _asbanana)
      (`self.K2_DestroyActor`))
    (:`then_2`
      (bind _asfalse_wall (cast `/Game/Blueprints/Pickups/FalseWall` OtherActor))
      (`/Game/Blueprints/Pickups/FalseWall.Despawn` _asfalse_wall)
      (`self.K2_DestroyActor`))
    (:`then_3`
      (bind _astarget_kart (cast `/Game/Blueprints/Pickups/TargetKart` OtherActor))
      (`self.K2_DestroyActor` _astarget_kart)
      (`self.K2_DestroyActor`))))

(fn `FindTarget`
  (returns (HomingTarget :type "SceneComponent Object Reference"))
  (bind _outactors (`GameplayStatics.GetAllActorsOfClassWithTag` "/Script/Engine.Actor" "Homing"))
  (for _array_element _outactors
    (bind _returnvalue (`KismetMathLibrary.VSize` (- (`self.K2_GetActorLocation` _array_element) (`self.K2_GetActorLocation`))))
    (if (< _returnvalue (`self.ClosestTarget`))
      (set `self.ClosestTarget` _returnvalue)
      (set `self.CurrentTarget` _array_element)))
  (return (`self.GetComponentByClass` (`self.CurrentTarget`) "/Script/Engine.SceneComponent")))

(fn `UserConstructionScript`)