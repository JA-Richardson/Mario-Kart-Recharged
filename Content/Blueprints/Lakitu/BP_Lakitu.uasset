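; BP_Lakitu is a Lakitu rescue actor that carries a Kart to a target location and rotation, then sets it alive again.
; After a short delay on BeginPlay, the Movement timeline moves itself and the kart together, with separate curves for horizontal travel, height and rotation.
; Rotation blends from the kart's current rotation each update along the shortest path.
; When the timeline finishes, it re-enables IsAlive and destroys itself after a delay.
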(event `self.ReceiveBeginPlay`
  (bind _defaultsceneroot (`self.DefaultSceneRoot`))
  (bind (_returnvalue_location _returnvalue_rotation) (`KismetMathLibrary.BreakTransform` (`self.GetTransform` (`self.Kart`))))
  ;[0.3005 0 1] Razvan Ivan - A0001151
  (set `self.StartLocation` (`SceneComponent.K2_GetComponentLocation` (`self.DefaultSceneRoot`)))
  (`KismetSystemLibrary.Delay` 1.0)
  (bind (_direction _trackz _trackxy _rotation) (`Timeline|Movement` :!via `PlayFromStart`)
    (:`Update`
      (`SceneComponent.K2_SetWorldLocation` _defaultsceneroot (`KismetMathLibrary.MakeVector` (`KismetMathLibrary.Lerp` (.x (`self.StartLocation`)) (.x (`self.TargetLocation`)) _trackxy) (`KismetMathLibrary.Lerp` (.y (`self.StartLocation`)) (.y (`self.TargetLocation`)) _trackxy) (`KismetMathLibrary.Lerp` (.z (`self.StartLocation`)) (.z (`self.TargetLocation`)) _trackz)) false false)
      (`SceneComponent.K2_SetWorldLocation` (`Actor.RootComponent` (`self.Kart`)) (`KismetMathLibrary.MakeVector` (`KismetMathLibrary.Lerp` (.x (`self.StartLocation`)) (.x (`self.TargetLocation`)) _trackxy) (`KismetMathLibrary.Lerp` (.y (`self.StartLocation`)) (.y (`self.TargetLocation`)) _trackxy) (`KismetMathLibrary.Lerp` (.z (`self.StartLocation`)) (.z (`self.TargetLocation`)) _trackz)) false false)
      (`SceneComponent.K2_SetWorldRotation` _defaultsceneroot (`KismetMathLibrary.RLerp` _returnvalue_rotation (`self.TargetRotation`) _rotation true) false false)
      (`SceneComponent.K2_SetWorldRotation` (`Actor.RootComponent` (`self.Kart`)) (`KismetMathLibrary.RLerp` _returnvalue_rotation (`self.TargetRotation`) _rotation true) false false))
    (:`Finished`
      (set `/Game/Blueprints/Kart/BP_Kart.isAlive` true (`self.Kart`))
      (`KismetSystemLibrary.Delay` 1.0)
      (`self.K2_DestroyActor`))))

(fn `UserConstructionScript`)