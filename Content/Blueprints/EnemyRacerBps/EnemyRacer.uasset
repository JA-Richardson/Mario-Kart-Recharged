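; An enemy racer actor that drives itself along the spline of a referenced track.
; On BeginPlay, if active, it runs a timeline with play rate set by a duration variable, mapping progress to spline distance to set world location and rotation each update.
; Pressing 1 toggles its camera between two relative offsets.
; A node randomizing the duration exists but is never executed.
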(event `Key|One`
  (params (Key :type "Key Structure"))
  (bind _camera1 (`self.Camera1`))
  (bind _camera1_2 (`self.Camera1`))
  (bind _returnvalue (`SceneComponent.GetRelativeTransform` _camera1))
  (bind _returnvalue_2 (`SceneComponent.GetRelativeTransform` _camera1_2))
  (:`Pressed`
    (`/Engine/EditorBlueprintResources/StandardMacros.FlipFlop`
      (:`A`
        (`SceneComponent.K2_SetRelativeLocation` _camera1_2 (`KismetMathLibrary.MakeVector` (- (.x (.location _returnvalue_2)) 600.0) (.y (.location _returnvalue_2)) (+ (.z (.location _returnvalue_2)) 100.0)) false false))
      (:`B`
        (`SceneComponent.K2_SetRelativeLocation` _camera1 (`KismetMathLibrary.MakeVector` (+ (.x (.location _returnvalue)) 600.0) (.y (.location _returnvalue)) (- (.z (.location _returnvalue)) 100.0)) false false)))))

(event `self.ReceiveBeginPlay`
  (if (`self.activecart`)
    (`self.movecart`)))

(event `movecart`
  (bind _returnvalue (`KismetMathLibrary.Lerp` 0.0 (`SplineComponent.GetSplineLength` (`/Game/Blueprints/EnemyRacerBps/TrackSpline.Spline` (`self.trackref`))) (`self.Alpha`)))
  (`TimelineComponent.SetPlayRate` (`self.Timeline_0`) (/ 1.0 (`self.duration/speed`)))
  (bind (_direction _newtrack_0) (`Timeline|Timeline_0` :!via `PlayFromStart`)
    (:`Update`
      (set `self.Alpha` _newtrack_0)
      (`self.K2_SetActorLocationAndRotation` (`SplineComponent.GetLocationAtDistanceAlongSpline` (`/Game/Blueprints/EnemyRacerBps/TrackSpline.Spline` (`self.trackref`)) _returnvalue "World") (`SplineComponent.GetRotationAtDistanceAlongSpline` (`/Game/Blueprints/EnemyRacerBps/TrackSpline.Spline` (`self.trackref`)) _returnvalue "World")))))

(fn `UserConstructionScript`)