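; Track spline actor from the enemy racer Blueprints, defining a path that can optionally be a closed loop.
; When ShowTrack is on, its construction script places a set number of scaled-down instanced static meshes at even distances along the spline.
; A Transform helper is meant to derive each instance's placement from spline location and rotation.
; The construction code is credited to Epic's Content Examples.
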(fn `UserConstructionScript`
  (locals (LastIndex :type Integer))
  (bind _number_of_meshes (`self.Number of meshes`))
  (`SplineComponent.SetClosedLoop` (`self.Spline`) (`self.ClosedLoop`) true)
  (if (`self.ShowTrack`)
    (if (> _number_of_meshes 0)
      (bind _output_get (set `local.LastIndex` (- _number_of_meshes 1)))
      (for _index (range (+ _output_get 1))
        (bind _returnvalue (* _index (/ (`SplineComponent.GetSplineLength` (`self.Spline`)) (`KismetMathLibrary.Conv_IntToDouble` (`local.LastIndex`)))))
        (`InstancedStaticMeshComponent.AddInstance` (`self.InstancedStaticMesh`) (`KismetMathLibrary.MakeTransform` (`KismetMathLibrary.InverseTransformLocation` (`self.GetTransform`) (`SplineComponent.GetLocationAtDistanceAlongSpline` (`self.Spline`) _returnvalue "World")) (`SplineComponent.GetRotationAtDistanceAlongSpline` (`self.Spline`) _returnvalue "Local") (`KismetMathLibrary.MakeVector` 0.0 0.0 0.0)))))))