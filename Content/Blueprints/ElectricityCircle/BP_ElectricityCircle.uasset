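; BP_ElectricityCircle is a short-lived pickup that grants electricity to the kart referenced by its Kart variable.
; On BeginPlay it traces down along its inverse up vector to snap onto the surface below, then destroys itself after a delay.
; When that specific kart overlaps the Hitbox, it increases the kart's electricity, has it spawn a boost circle and destroys itself.
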(event `self.ReceiveBeginPlay`
  (bind _defaultsceneroot (`self.DefaultSceneRoot`))
  (bind _returnvalue (`SceneComponent.K2_GetComponentLocation` _defaultsceneroot))
  ;[0.3005 0 1] Razvan Ivan - A0001151
  (`|ExecutionSequence`
    (:`then_0`
      (bind (_outhit _returnvalue_2) (`KismetSystemLibrary.LineTraceSingle` _returnvalue (+ _returnvalue (* (`SceneComponent.GetUpVector` _defaultsceneroot) -1000.0)) "TraceTypeQuery1"))
      (if _returnvalue_2
        (`SceneComponent.K2_SetWorldLocation` (`self.DefaultSceneRoot`) (`.Location` (`GameplayStatics.BreakHitResult` _outhit)) false false)))
    (:`then_1`
      (`KismetSystemLibrary.Delay` 5.0)
      (`self.K2_DestroyActor`))))

(event `self.hitbox.OnComponentBeginOverlap`
  (params (OverlappedComponent :type "PrimitiveComponent Object Reference") (OtherActor :type "Actor Object Reference") (OtherComp :type "PrimitiveComponent Object Reference") (OtherBodyIndex :type Integer) (bFromSweep :type Boolean) (SweepResult :type "HitResult Structure (by ref)"))
  ;[0.3005 0 1] Razvan Ivan - A0001151
  (bind _asbp_kart (cast `/Game/Blueprints/Kart/BP_Kart` OtherActor))
  (if (== _asbp_kart (`self.Kart`))
    (`/Game/Blueprints/Kart/BP_Kart.Increase Electricity` _asbp_kart 5.0)
    (`/Game/Blueprints/Kart/BP_Kart.SpawnBoostCircle` _asbp_kart)
    (`self.K2_DestroyActor`)))

(fn `UserConstructionScript`)