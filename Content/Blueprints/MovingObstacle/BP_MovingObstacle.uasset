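; Moving obstacle actor that travels between its starting position and a target point, repeating for as long as it exists.
; On BeginPlay it stores its world location and turns TargetPosition, an offset scaled by the root's relative scale, into a world-space target.
; A timeline drives a non-swept location lerp between the two points and restarts from the beginning whenever it finishes.
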(event `self.ReceiveBeginPlay`
  (bind _defaultsceneroot (`self.DefaultSceneRoot`))
  (bind (_targetposition_x _targetposition_y _targetposition_z) (`KismetMathLibrary.BreakVector` (`self.TargetPosition`)))
  (bind _returnvalue (`SceneComponent.K2_GetComponentLocation` _defaultsceneroot))
  (bind (_relativescale3d_x _relativescale3d_y _relativescale3d_z) (`KismetMathLibrary.BreakVector` (`SceneComponent.RelativeScale3D` _defaultsceneroot)))
  ;[0.3005 0 1] Razvan Ivan - A0001151
  (set `self.OriginalPosition` _returnvalue)
  (set `self.TargetPosition` (+ _returnvalue (`KismetMathLibrary.MakeVector` (* _targetposition_x _relativescale3d_x) (* _targetposition_y _relativescale3d_y) (* _targetposition_z _relativescale3d_z))))
  (bind (_direction _lerp) (`Timeline|Timeline` :!label _label)
    (:`Update`
      (`SceneComponent.K2_SetWorldLocation` (`self.DefaultSceneRoot`) (`KismetMathLibrary.VLerp` (`self.OriginalPosition`) (`self.TargetPosition`) _lerp) false false))
    (:`Finished`
      (goto _label :!via `PlayFromStart`))))

(fn `UserConstructionScript`)