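; Player controller for the kart game that sets up the player's UI and passes input to the kart.
; On BeginPlay it creates the HUD and pause widgets, possesses the first BP_Kart found, hands it the HUD and calls 321GO on it.
; Drive, steer, boost, drift and pickup inputs are forwarded to the kart through a ValidKart validity macro.
; PauseGame toggles the pause menu, game pause, mouse cursor and input mode.
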(event `self.ReceiveBeginPlay`
  (`|ExecutionSequence`
    (:`then_0`
      (bind _returnvalue (`|CreateWidget` "/Game/Interface/Menu/HUD/HUD_Widget.HUD_Widget_C" null 0.0 0.5 null))
      (bind _output_get (set `self.HUD` _returnvalue))
      (`UserWidget.AddToViewport` _output_get 0))
    (:`then_1`
      (bind _returnvalue_2 (`|CreateWidget` "/Game/Interface/Menu/PauseMenu/PauseWidget.PauseWidget_C"))
      (set `self.PauseMenu` _returnvalue_2))
    (:`then_2`
      ;[0.3005 0 1] Razvan Ivan - A0001151
      (bind _outactors (`GameplayStatics.GetAllActorsOfClass` "/Game/Blueprints/Kart/BP_Kart.BP_Kart_C"))
      (bind _output_get_2 (set `self.Kart` (`|GetArrayItem` _outactors)))
      (`self.Possess` _output_get_2)
      (bind _output_get_3 (set `/Game/Blueprints/Kart/BP_Kart.HUD` (`self.HUD`) (`self.Kart`)))
      (`/Game/Interface/Menu/HUD/HUD_Widget.321GO` _output_get_3))))

(event `InputAction|Boost`
  (params (Key :type "Key Structure"))
  ;[0.3005 0 1] Razvan Ivan - A0001151
  (:`Pressed`
    (bind _kart (`self.ValidKart`)
      (:`Valid`
        (`/Game/Blueprints/Kart/BP_Kart.Boost` _kart true))))
  (:`Released`
    (bind _kart_2 (`self.ValidKart`)
      (:`Valid`
        (`/Game/Blueprints/Kart/BP_Kart.Boost` _kart_2 false)))))

(event `InputAction|UsePickup`
  (params (Key :type "Key Structure"))
  ;[0.3005 0 1] Razvan Ivan - A0001151
  (:`Pressed`
    (bind _kart (`self.ValidKart`)
      (:`Valid`
        (`/Game/Blueprints/Kart/BP_Kart.UsePickup` _kart)))))

(event `InputAction|SwapPickup`
  (params (Key :type "Key Structure"))
  ;[0.3005 0 1] Razvan Ivan - A0001151
  (:`Pressed`
    (bind _kart (`self.ValidKart`)
      (:`Valid`
        (`/Game/Blueprints/Kart/BP_Kart.SwapPickups` _kart)))))

(event `InputAxis|ForwardInput`
  (params (AxisValue :type "Float (single-precision)"))
  ;[0.3005 0 1] Razvan Ivan - A0001151
  (bind _kart (`self.ValidKart`)
    (:`Valid`
      (`/Game/Blueprints/Kart/BP_Kart.MoveKart` _kart AxisValue))))

(event `InputAction|Pause Game`
  (params (Key :type "Key Structure"))
  ;[0.3005 0 1] Razvan Ivan - A0001151
  (:`Pressed`
    (`self.PauseGame`)))

(event `InputAxis|TurnAround`
  (params (AxisValue :type "Float (single-precision)"))
  ;[0.3005 0 1] Razvan Ivan - A0001151
  (bind _kart (`self.ValidKart`)
    (:`Valid`
      (`/Game/Blueprints/Kart/BP_Kart.SteerKart` _kart AxisValue))))

(event `InputAction|Drift`
  (params (Key :type "Key Structure"))
  ;[0.3005 0 1] Razvan Ivan - A0001151
  (:`Pressed`
    (bind _kart (`self.ValidKart`)
      (:`Valid`
        (`/Game/Blueprints/Kart/BP_Kart.BeginDrift` _kart (stale `InputAxis|TurnAround` AxisValue)))))
  (:`Released`
    (bind _kart_2 (`self.ValidKart`)
      (:`Valid`
        (`/Game/Blueprints/Kart/BP_Kart.EndDrift` _kart_2)))))

(fn `PauseGame`
  (bind _pausemenu (`self.PauseMenu`))
  (if (`GameplayStatics.IsGamePaused`)
    (`Widget.RemoveFromParent` _pausemenu)
    (`GameplayStatics.SetGamePaused` false)
    (set `self.bShowMouseCursor` false)
    (`WidgetBlueprintLibrary.SetInputMode_GameOnly` null)
    (else
      (`UserWidget.AddToViewport` _pausemenu 0)
      (`GameplayStatics.SetGamePaused` true)
      (set `self.bShowMouseCursor` true)
      (`WidgetBlueprintLibrary.SetInputMode_GameAndUIEx` self _pausemenu))))

(fn `UserConstructionScript`)