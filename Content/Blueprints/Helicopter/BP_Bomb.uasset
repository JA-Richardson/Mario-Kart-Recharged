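; BP_Bomb is a helicopter-related bomb actor that stuns any BP_Kart overlapping its hitbox.
; On a kart hit it calls StunKart, activates the explosion effect, disables collision and destroys the hitbox so it cannot trigger again.
; A timer started at BeginPlay destroys the actor after a few seconds regardless, so it also cuts short the equal delayed destroy that follows a hit.
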(event `self.ReceiveBeginPlay`
  (`KismetSystemLibrary.Delay` 5.0)
  (`self.K2_DestroyActor`))

(event `self.Hitbox.OnComponentBeginOverlap`
  (params (OverlappedComponent :type "PrimitiveComponent Object Reference") (OtherActor :type "Actor Object Reference") (OtherComp :type "PrimitiveComponent Object Reference") (OtherBodyIndex :type Integer) (bFromSweep :type Boolean) (SweepResult :type "HitResult Structure (by ref)"))
  (bind _asbp_kart (cast `/Game/Blueprints/Kart/BP_Kart` OtherActor))
  (`/Game/Blueprints/Kart/BP_Kart.StunKart` _asbp_kart 0.01)
  (`ActorComponent.Activate` (`self.Explosion`) false)
  (`self.SetActorEnableCollision` false)
  (`ActorComponent.K2_DestroyComponent` (`self.Hitbox`))
  (`KismetSystemLibrary.Delay` 5.0)
  (`self.K2_DestroyActor`))

(fn `UserConstructionScript`)