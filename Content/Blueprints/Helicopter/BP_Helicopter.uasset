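; Helicopter actor that hovers around its spawn point and repeatedly drops bombs.
; BeginPlay stores the original transform and starts looping timers for bomb spawning, movement and rotation.
; Movement and rotation timelines lerp toward random offsets around that original transform, so the wobble never drifts away.
; Each BP_Bomb is pushed along a random downward cone, and Tick spins the blade at a fixed, frame-rate-dependent step.
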(event `self.ReceiveBeginPlay`
  ;[0.3005 0 1] Razvan Ivan - A0001151
  (`|ExecutionSequence`
    (:`then_0`
      (set `self.Original` (`SceneComponent.K2_GetComponentLocation` (`self.DefaultSceneRoot`)))
      (set `self.OriginalRotation` (`SceneComponent.K2_GetComponentRotation` (`self.DefaultSceneRoot`))))
    (:`then_1`
      (`KismetSystemLibrary.K2_SetTimerDelegate` (delegate `SpawnMeteor`) 2.0 true)
      (`KismetSystemLibrary.K2_SetTimerDelegate` (delegate `MoveHelicopter`) 1.0 true)
      (`KismetSystemLibrary.K2_SetTimerDelegate` (delegate `RotateHelicopter`) 0.5 true))))

(event `SpawnMeteor`
  ;[0.3005 0 1] Razvan Ivan - A0001151
  (bind _returnvalue (`|SpawnActorFromClass` "/Game/Blueprints/Helicopter/BP_Bomb.BP_Bomb_C" (`KismetMathLibrary.MakeTransform` (.location (`SceneComponent.K2_GetComponentToWorld` (`self.DefaultSceneRoot`))) (.rotation (`SceneComponent.K2_GetComponentToWorld` (`self.DefaultSceneRoot`)))) "Undefined" "OverrideRootScale" null null))
  (`PrimitiveComponent.AddForce` (`/Game/Blueprints/Helicopter/BP_Bomb.Sphere` _returnvalue) (* (`KismetMathLibrary.RandomUnitVectorInConeInDegrees` (0.0 0.0 -1.0) 50.0) 200000.0) "None" true))

(event `MoveHelicopter`
  ;[0.3005 0 1] Razvan Ivan - A0001151
  (set `self.CurrentLocation` (`SceneComponent.K2_GetComponentLocation` (`self.DefaultSceneRoot`)))
  (set `self.TargetLocation` (`self.GetRandomPosition`))
  (bind (_direction _flight) (`Timeline|Timeline_0` :!via `PlayFromStart`)
    (:`Update`
      (`SceneComponent.K2_SetWorldLocation` (`self.DefaultSceneRoot`) (`KismetMathLibrary.VLerp` (`self.CurrentLocation`) (`self.TargetLocation`) _flight) false false))))

(event `RotateHelicopter`
  ;[0.3005 0 1] Razvan Ivan - A0001151
  (set `self.CurrentRotation` (`SceneComponent.K2_GetComponentRotation` (`self.DefaultSceneRoot`)))
  (set `self.TargetRotation` (`self.GetRandomRotation`))
  (bind (_direction _rotation) (`Timeline|Timeline_1` :!via `PlayFromStart`)
    (:`Update`
      (`SceneComponent.K2_SetWorldRotation` (`self.DefaultSceneRoot`) (`KismetMathLibrary.RLerp` (`self.CurrentRotation`) (`self.TargetRotation`) _rotation true) false false))))

(event `self.ReceiveTick`
  (params (DeltaSeconds :type "Float (single-precision)"))
  (`SceneComponent.K2_AddRelativeRotation` (`self.Blade`) (`KismetMathLibrary.MakeRotator` 0.0 0.0 1200.0) false false))

(fn `GetRandomPosition`
  (returns (Result :type "Vector Structure"))
  (bind _returnvalue (`KismetMathLibrary.RandomFloatInRange` -200.0 200.0))
  ;[0.3005 0 1] Razvan Ivan - A0001151
  (return (+ (`self.Original`) (`KismetMathLibrary.MakeVector` _returnvalue _returnvalue (`KismetMathLibrary.RandomFloatInRange` -100.0 100.0)))))

(fn `GetRandomRotation`
  (returns (Result :type "Rotator Structure"))
  ;[0.3005 0 1] Razvan Ivan - A0001151
  (return (`KismetMathLibrary.MakeRotator` (+ (`KismetMathLibrary.RandomFloatInRange` -3.0 3.0) (.roll (`self.OriginalRotation`))) (+ (`KismetMathLibrary.RandomFloatInRange` -3.0 3.0) (.pitch (`self.OriginalRotation`))) (+ (`KismetMathLibrary.RandomFloatInRange` -3.0 3.0) (.yaw (`self.OriginalRotation`))))))

(fn `UserConstructionScript`)